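; Fish character that flops around by launching itself in randomized directions, with particles on each launch and a sound on landing.
; Flutter launches it only when grounded and in the required state; the flutter state times out to idle with a final launch.
; Physical animation and partial-body simulation loosen the mesh, whose animation pauses when idle.
; Tick aligns the mesh to velocity, and possession triggers an initial launch and moves the audio listener onto the fish.
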(event Custom|Flutter
  (bind _returnvalue (CallFunction|CheckFluttable))
  (if _returnvalue
    (CallFunction|FlutterFish)))

(event Custom|EventSetIdle
  (Variables|Default|SetCurState "WAITFORIDLE")
  (CallFunction|LastDance)
  (CallFunction|SetSimulatePhysicsBelow true)
  (Variables|/Script/Engine.SkeletalMeshComponent|SetbPauseAnims (Variables|Character|GetMesh) true))

(event Custom|EventSetFlutter
  (Variables|Default|SetCurState "FLUTTER")
  (CallFunction|SetSimulatePhysicsBelow true)
  (Variables|/Script/Engine.SkeletalMeshComponent|SetbPauseAnims (Variables|Character|GetMesh) false)
  (Utilities|Time|SetTimerbyFunctionName 0 "EventSetIdle" 3.0))

(event EventBeginPlay
  (Class|PhysicalAnimationComponent|SetSkeletalMeshComponent (Variables|Default|GetPhysicalAnimation) (Variables|Character|GetMesh))
  (Class|PhysicalAnimationComponent|ApplyPhysicalAnimationSettingsBelow (Variables|Default|GetPhysicalAnimation) (Variables|Default|GetBodyName1) (Variables|Default|GetPhysical%20Animation%20Data) true)
  (Class|PhysicalAnimationComponent|ApplyPhysicalAnimationSettingsBelow (Variables|Default|GetPhysicalAnimation) (Variables|Default|GetBodyName2) (Variables|Default|GetPhysical%20Animation%20Data) true))

(event EventTick
  (params (DeltaSeconds :type Float%20%28single-precision%29))
  (bind _returnvalue (Transformation|GetVelocity))
  (bind _returnvalue_2 (Math|Conversions|RotationFromXVector _returnvalue))
  (if (> (Math|Vector|VectorLength _returnvalue) 0.0)
    (Transformation|SetWorldRotation (Variables|Character|GetMesh) (Math|Rotator|MakeRotator (+ (.roll _returnvalue_2) 9e+01) (.pitch _returnvalue_2) (.yaw _returnvalue_2)) false false)))

(event EventPossessed
  (params (NewController :type Controller%20Object%20Reference))
  (Utilities|FlowControl|Delay 0.0)
  (CallFunction|InitializeCharacter)
  (bind _asplayer_controller (Utilities|Casting|CastToPlayerController (Pawn|GetController)))
  (Class|PlayerController|SetAudioListenerOverride _asplayer_controller (Variables|Transformation|GetRootComponent) "0, 0, 0" "0, 0, 0"))

(event EventOnLanded
  (params (Hit :type Hit%20Result%20Structure%20%28by%20ref%29))
  (Audio|PlaySound2D (Variables|Default|GetFlutterSound) 1.0 1.0 0.0 0 0))

(fn ConstructionScript)

(fn DrawDebugFlutterLine
  (bind _mesh (Variables|Character|GetMesh))
  (bind _randomflutterrollmax (Variables|Default|GetRandomFlutterRollMax))
  (bind _randomflutterpitchmax (Variables|Default|GetRandomFlutterPitchMax))
  (bind _returnvalue (Transformation|GetWorldLocation _mesh))
  (Rendering|Debug|DrawDebugLine _returnvalue (+ _returnvalue (* (Math|Vector|Normalize (Math|Vector|RotateVector (Math|Vector|GetRightVector _mesh) (Math|Rotator|MakeRotator (Math|Random|RandomFloatinRange (* _randomflutterrollmax -1.0) _randomflutterrollmax) (Math|Random|RandomFloatinRange (* _randomflutterpitchmax -1.0) _randomflutterpitchmax) 0.0))) (Math|Random|RandomFloatinRange (Variables|Default|GetRandomFlutterStrengthMin) (Variables|Default|GetRandomFlutterStrengthMax)))) "(R=1.000000,G=0.000000,B=0.000000,A=1.000000)" 2.0 2.0))

(fn FlutterFish
  (bind _randomflutterrollmax (Variables|Default|GetRandomFlutterRollMax))
  (bind _randomflutterpitchmin (Variables|Default|GetRandomFlutterPitchMin))
  (bind _randomflutterpitchmax (Variables|Default|GetRandomFlutterPitchMax))
  (bind _randomflutterrollmin (Variables|Default|GetRandomFlutterRollMin))
  (bind _returnvalue (Math|Random|RandomFloatinRange _randomflutterpitchmin _randomflutterpitchmax))
  (bind _returnvalue_2 (Math|Random|RandomFloatinRange _randomflutterrollmin _randomflutterrollmax))
  (if (< (- (Math|Random|RandomFloatinRange 0.0 1.0) 0.5) 0.0)
    (Variables|Default|SetRandomFlutterRoll (* _returnvalue_2 -1.0))
    (else
      (Variables|Default|SetRandomFlutterRoll _returnvalue_2)))
  (if (< (- (Math|Random|RandomFloatinRange 0.0 1.0) 0.5) 0.0)
    (Variables|Default|SetRandomFlutterPitch (* _returnvalue -1.0))
    (else
      (Variables|Default|SetRandomFlutterPitch _returnvalue)))
  (Character|LaunchCharacter (* (Math|Vector|RotateVector (Variables|Default|GetFlutterVec) (Math|Rotator|MakeRotator (Variables|Default|GetRandomFlutterRoll) (Variables|Default|GetRandomFlutterPitch) 0.0)) (Math|Random|RandomFloatinRange (Variables|Default|GetRandomFlutterStrengthMin) (Variables|Default|GetRandomFlutterStrengthMax))) true true)
  (Components|Activation|Activate (Variables|Default|GetFlutterParticle) true))

(fn SetSimulatePhysicsBelow
  (params (bSimulate :type Boolean))
  (Class|SkeletalMeshComponent|SetAllBodiesBelowSimulatePhysics (Variables|Character|GetMesh) (Variables|Default|GetBodyName1) bSimulate false)
  (Class|SkeletalMeshComponent|SetAllBodiesBelowSimulatePhysics (Variables|Character|GetMesh) (Variables|Default|GetBodyName2) bSimulate false))

(fn CheckFluttable
  (return (and (not (AI|Components|NavMovement|IsFalling (Variables|Character|GetCharacterMovement))) (== (Variables|Default|GetCurState) 1))))

(fn LastDance
  (Character|LaunchCharacter (* (Math|Vector|RotateVector (Variables|Default|GetFlutterVec) (Math|Rotator|MakeRotator (Math|Random|RandomFloatinRange -3e+01 3e+01) (Math|Random|RandomFloatinRange -3e+01 3e+01) 0.0)) 5e+02) true true)
  (Components|Activation|Activate (Variables|Default|GetFlutterParticle) true))

(fn InitializeCharacter
  (Variables|Default|SetCurState "WAITFORIDLE")
  (Character|LaunchCharacter (* (Math|Vector|RotateVector "0.000000,0.000000,-1.000000" (Math|Rotator|MakeRotator 3e+01 0.0 0.0)) 3e+02) true true)
  (CallFunction|SetSimulatePhysicsBelow true)
  (Variables|/Script/Engine.SkeletalMeshComponent|SetbPauseAnims (Variables|Character|GetMesh) true))