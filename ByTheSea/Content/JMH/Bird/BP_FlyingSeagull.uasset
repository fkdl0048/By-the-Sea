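; Seagull actor that flies along the path of a BP_Spline actor in the level.
; On BeginPlay it finds that spline with GetActorOfClass and starts a Timeline whose play rate derives from TimeToComplete.
; Each update maps the timeline track to distance along the spline and sets the actor's transform, taking location in world space but rotation in local space.
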(event Custom|MoveObject
  (bind _spline_ref (Variables|Default|GetSpline%20Ref))
  (bind _spline (Variables|/Game/JMH/Bird/BP_Spline.BP_Spline_C|GetSpline _spline_ref))
  (Components|Timeline|SetPlayRate (Variables|Default|GetTimeline) (/ 1.0 (Variables|Default|GetTimeToComplete)))
  (bind _newtrack_0 (Timeline|Timeline Play)
    (:Update
      (Transformation|SetActorTransform (Math|Transform|MakeTransform (Spline|GetLocationatDistanceAlongSpline _spline (Math|Float|Lerp 0.0 (Spline|GetSplineLength (Variables|/Game/JMH/Bird/BP_Spline.BP_Spline_C|GetSpline (Variables|Default|GetSpline%20Ref))) _newtrack_0) "World") (Spline|GetRotationatDistanceAlongSpline _spline (Math|Float|Lerp 0.0 (Spline|GetSplineLength (Variables|/Game/JMH/Bird/BP_Spline.BP_Spline_C|GetSpline (Variables|Default|GetSpline%20Ref))) _newtrack_0) "Local") "1.000000,1.000000,1.000000")))))

(event EventBeginPlay
  (bind _returnvalue (Actor|GetActorOfClass "/Game/JMH/Bird/BP_Spline.BP_Spline_C"))
  (Variables|Default|SetSpline%20Ref _returnvalue)
  (CallFunction|MoveObject))

(fn ConstructionScript)